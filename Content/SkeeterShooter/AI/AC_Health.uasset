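; Health component for Skeeter Shooter AI that resolves gun hits against a shield and health pool.
; TakeDamage classifies hits by critical bone or shield, then derives damage from the gun's first-shot and headshot values.
; Non-lethal damage drains shield before health, with Health -1 skipping depletion, while kills zero both and send KillMessage to the owner.
; A damage indicator actor spawns unless the GameState hides damage; the hit sound function is an empty stub.
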(event EventBeginPlay)

(event EventTick
  (params (DeltaSeconds :type Float%20%28single-precision%29)))

(event EventTakeDamage
  (params (Hit%20Screen%20Location :type Vector%202D%20Structure) (Hit :type Hit%20Result%20Structure) (Current%20Gun :type S%20Gun%20Structure) (First%20Shot :type Boolean))
  (Variables|Default|SetHit Hit)
  (Variables|Default|SetCurrent%20Gun Current%20Gun)
  (if (not (Variables|Default|GetKilled))
    (bind _hit_type (CallFunction|CalculateHitType (Variables|Default|GetHit)))
    (bind (_damage_to_take _killed) (CallFunction|CalculateDamage _hit_type (Variables|Default|GetCurrent%20Gun) First%20Shot))
    (Variables|Default|SetKilled _killed)
    (if (Variables|Default|GetKilled)
      (Variables|Default|SetShield 0)
      (Variables|Default|SetHealth 0)
      (Utilities|FlowControl|Sequence
        (:then_1
          (bind _asgs_skeeter_shooter (Utilities|Casting|CastToGS_SkeeterShooter (Game|GetGameState) :!label _label))
          (bind _hide_damage (Default|GetHideDamage _asgs_skeeter_shooter))
          (if (not _hide_damage)
            (CallFunction|SpawnDamageIndicator _damage_to_take _hit_type Hit%20Screen%20Location (Variables|Default|GetHit))
            (CallFunction|HitSound (stale _broke_shield) _hit_type)))
        (:then_2
          (Class|BPIInteraction|Kill(Message) (Components|GetOwner) (Variables|Default|GetHit) (Variables|Default|GetCurrent%20Gun))))
      (elif (== (Variables|Default|GetHealth) -1)
        (goto _label)
        (else
          (bind _broke_shield (CallFunction|ApplyDamage _hit_type _damage_to_take))
          (goto _label))))))

(fn CalculateHitType
  (params (Hit :type Hit%20Result%20Structure))
  (LocalVariables|SetHit%20Type%20Local (select (> (Variables|Default|GetShield) 0) "NewEnumerator2" "NewEnumerator0"))
  (for _array_element (Variables|Default|GetCritical%20Bones)
    (if (== _array_element (.HitBoneName (Collision|BreakHitResult Hit)))
      (bind _output_get (LocalVariables|SetHit%20Type%20Local "NewEnumerator1"))
      (return _output_get)))
  (return (LocalVariables|GetHit%20Type%20Local)))

(fn CalculateDamage
  (params (Hit%20Type :type E_HitTypes%20Enum :default "NewEnumerator0") (Current%20Gun :type S%20Gun%20Structure) (First%20Shot :type Boolean))
  (bind (_gunname _ammotype _minimumspread _firstshotdelay _hipfirerates _firstshotdamage _damage _firstshotheadshotmultiplier _headshotmultiplier) (Utilities|Struct|BreakS_Gun Current%20Gun))
  (bind _returnvalue (Utilities|Enum|Equal(Enum) Hit%20Type "NewEnumerator1"))
  (bind _shield (Variables|Default|GetShield))
  (bind _health (Variables|Default|GetHealth))
  (bind _health_2 (Variables|Default|GetHealth))
  (bind _returnvalue_2 (Math|Integer|SelectInt _firstshotdamage _damage First%20Shot))
  (bind _returnvalue_3 (Math|Float|SelectFloat _firstshotheadshotmultiplier _headshotmultiplier First%20Shot))
  (bind _returnvalue_4 (== _health_2 -1))
  (bind _returnvalue_5 (Math|Integer|SelectInt 100000 _health _returnvalue_4))
  (bind _returnvalue_6 (* _returnvalue_2 _returnvalue_3))
  (bind _returnvalue_7 (Math|Float|Round _returnvalue_6))
  (bind _returnvalue_8 (+ _shield _returnvalue_5))
  (bind _returnvalue_9 (Math|Integer|SelectInt _returnvalue_7 _returnvalue_2 _returnvalue))
  (bind _returnvalue_10 (- _returnvalue_8 _returnvalue_9))
  (bind _returnvalue_11 (<= _returnvalue_10 0))
  (return (Math|Integer|SelectInt (+ (Variables|Default|GetShield) (Variables|Default|GetHealth)) _returnvalue_9 _returnvalue_11) _returnvalue_11))

(fn ApplyDamage
  (params (Hit%20Type :type E_HitTypes%20Enum :default "NewEnumerator0") (Damage :type Integer))
  (LocalVariables|SetDamage%20Local Damage)
  (Utilities|FlowControl|Sequence
    (:then_0
      (LocalVariables|SetHas%20Shield%20Local (> (Variables|Default|GetShield) 0))
      (if (<= (- (Variables|Default|GetShield) (LocalVariables|GetDamage%20Local)) 0)
        (LocalVariables|SetDamage%20Local (Math|Integer|Absolute(Integer) (- (Variables|Default|GetShield) (LocalVariables|GetDamage%20Local))))
        (LocalVariables|SetBroke%20Shield%20Local (LocalVariables|GetHas%20Shield%20Local))
        (LocalVariables|SetHas%20Shield%20Local false)
        (Variables|Default|SetShield 0)
        (else
          (Variables|Default|SetShield (- (Variables|Default|GetShield) (LocalVariables|GetDamage%20Local)))
          (return (LocalVariables|GetBroke%20Shield%20Local)))))
    (:then_1
      (Variables|Default|SetHealth (- (Variables|Default|GetHealth) (LocalVariables|GetDamage%20Local)))
      (return (LocalVariables|GetBroke%20Shield%20Local)))))

(fn SpawnDamageIndicator
  (params (Damage :type Integer) (Hit%20Type :type E_HitTypes%20Enum :default "NewEnumerator0") (Screen%20Location :type Vector%202D%20Structure) (Hit :type Hit%20Result%20Structure))
  (Game|SpawnActorfromClass "/Game/SkeeterShooter/UI/HeadshotIndicator.HeadshotIndicator_C" (Math|Transform|MakeTransform (.Location (Collision|BreakHitResult Hit)) "0, 0, 0" "1.000000,1.000000,1.000000") "Undefined" "MultiplyWithRoot" 0 Hit%20Type Damage Screen%20Location 0))

(fn HitSound
  (params (Broke%20Shield :type Boolean) (Hit%20Type :type E_HitTypes%20Enum :default "NewEnumerator0"))
  (return))