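; Test AI enemy character for SkeeterShooter that randomizes its variant on spawn and handles its own death.
; BeginPlay randomly picks a smaller size and either a Manny mesh with shield or the default mesh with set health, adjusting walk speed for each combination.
; Kill ragdolls the mesh with a clamped, lifted impulse at the hit bone scaled by gun kick, then a timeline animates its scale before destroying the actor.
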(event EventKill
  (params (Hit :type Hit%20Result%20Structure) (Current%20Gun :type S%20Gun%20Structure))
  (bind _shootkick (Utilities|Struct|BreakS_Gun Current%20Gun))
  (bind (_bblockinghit _binitialoverlap _time _distance _location _impactpoint _normal _impactnormal _physmat _hitactor _hitcomponent _hitbonename _bonename) (Collision|BreakHitResult Hit))
  (bind _returnvalue (* _impactnormal -100 _shootkick))
  (Physics|SetSimulatePhysics (Variables|Character|GetMesh) true)
  (Pawn|Components|CharacterMovement|DisableMovement (Variables|Character|GetCharacterMovement))
  (Physics|AddImpulse (Variables|Character|GetMesh) (Math|Vector|VectorClampSizeMax (Math|Vector|MakeVector (.x _returnvalue) (.y _returnvalue) (+ (.z _returnvalue) 1e+03)) 1.5e+03) _bonename true)
  (Utilities|FlowControl|Delay 0.5)
  (bind _alpha (Timeline|Timeline PlayFromStart)
    (:Update
      (Transformation|SetWorldScale3D (Variables|Character|GetMesh) (Math|Conversions|ToVector(Float) _alpha)))
    (:Finished
      (Actor|DestroyActor))))

(event EventBeginPlay
  (bind _output_get (Variables|Default|SetSmall (Utilities|Select :Index (Math|Random|RandomIntegerinRange 0 6) :Option%200 false :Option%201 false :Option%202 false :Option%203 false :Option%204 false :Option%205 true :Option%206 true)))
  (if _output_get
    (Transformation|SetWorldScale3D (Variables|Character|GetMesh) "0.750000,0.750000,0.750000"))
  (if (Utilities|Select :Index (Math|Random|RandomIntegerinRange 0 4) :Option%200 false :Option%201 false :Option%202 false :Option%203 true :Option%204 true)
    (Components|SkeletalMesh|SetSkeletalMeshAsset (Variables|Character|GetMesh) "/Game/Characters/Mannequins/Meshes/SKM_Manny.SKM_Manny")
    (Variables|/Game/SkeeterShooter/AI/AC_Health.AC_Health_C|SetShield (Variables|Default|GetAC_Health) (Math|Integer|SelectInt 50 100 (Variables|Default|GetSmall)))
    (if (Variables|Default|GetSmall)
      (Variables|/Script/Engine.CharacterMovementComponent|SetMaxWalkSpeed (Variables|Character|GetCharacterMovement) (Math|Random|RandomFloatinRange 1.5e+02 2e+02))
      (else
        (Variables|/Script/Engine.CharacterMovementComponent|SetMaxWalkSpeed (Variables|Character|GetCharacterMovement) (Math|Random|RandomFloatinRange 125.0 175.0))))
    (elif (Variables|Default|GetSmall)
      (Variables|/Script/Engine.CharacterMovementComponent|SetMaxWalkSpeed (Variables|Character|GetCharacterMovement) (Utilities|Select :Index (Math|Random|RandomIntegerinRange 0 3) :Option%200 1.5e+02 :Option%201 175.0 :Option%202 2e+02 :Option%203 225.0))
      (Variables|/Game/SkeeterShooter/AI/AC_Health.AC_Health_C|SetHealth (Variables|Default|GetAC_Health) 75)
      (else
        (Variables|/Script/Engine.CharacterMovementComponent|SetMaxWalkSpeed (Variables|Character|GetCharacterMovement) (Utilities|Select :Index (Math|Random|RandomIntegerinRange 0 2) :Option%200 2e+02 :Option%201 225.0 :Option%202 2.5e+02))
        (Variables|/Game/SkeeterShooter/AI/AC_Health.AC_Health_C|SetHealth (Variables|Default|GetAC_Health) 100)))))

(fn ConstructionScript)