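; BP_TV is an interactable television actor that toggles on and off.
; BeginPlay creates dynamic material instances for the case and screen slots.
; Interacting with the Button component flips the On state, setting screen emissive intensity, RectLight intensity and the button's pressed offset.
; Interacting with any other component plays a sped-up timeline that animates the root's scale.
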(event EventBeginPlay
  (bind _tv (Variables|Default|GetTV))
  (bind _tv_2 (Variables|Default|GetTV))
  (Components|Timeline|SetPlayRate (Variables|Default|GetTimeline) 4.0)
  (bind _returnvalue (Rendering|Material|CreateDynamicMaterialInstance _tv_2 0 (Rendering|Material|GetMaterial _tv_2 0) "None" :!class /Script/Engine.PrimitiveComponent))
  (bind _output_get (Variables|Default|SetTV%20Case _returnvalue))
  (Rendering|Material|SetMaterial _tv_2 0 _output_get)
  (bind _returnvalue_2 (Rendering|Material|CreateDynamicMaterialInstance _tv 1 (Rendering|Material|GetMaterial _tv 1) "None" :!class /Script/Engine.PrimitiveComponent))
  (bind _output_get_2 (Variables|Default|SetTV%20Screen _returnvalue_2))
  (Rendering|Material|SetMaterial _tv 1 _output_get_2))

(event EventTick
  (params (DeltaSeconds :type Float%20%28single-precision%29)))

(event EventInteract
  (params (Hit%20Component :type Primitive%20Component%20Object%20Reference))
  (if (== Hit%20Component (Variables|Default|GetButton))
    (Variables|Default|SetOn (not (Variables|Default|GetOn)))
    (Rendering|Material|SetScalarParameterValue (Variables|Default|GetTV%20Screen) "Emissive Intensity" (Math|Float|SelectFloat 2.0 0.0 (Variables|Default|GetOn)) :!class /Script/Engine.MaterialInstanceDynamic)
    (Rendering|Components|Light|SetIntensity (Variables|Default|GetRectLight) (Math|Float|SelectFloat 5.0 0.0 (Variables|Default|GetOn)))
    (Transformation|SetRelativeLocation (Variables|Default|GetButton) (Math|Vector|MakeVector (Math|Float|SelectFloat 1.0 0.0 (Variables|Default|GetOn)) 0.0 0.0) false false)
    (else
      (bind _scale (Timeline|Timeline PlayFromStart)
        (:Update
          (Transformation|SetRelativeScale3D (Variables|Default|GetDefaultSceneRoot) (Math|Conversions|ToVector(Float) _scale)))))))

(fn ConstructionScript)

(fn GetCanInteract
  (return true))