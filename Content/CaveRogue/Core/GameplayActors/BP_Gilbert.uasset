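; BP_Gilbert is an interactable actor that plays a quick height and scale animation on its mesh when interacted with.
; Interact restarts a Timeline, sped up at BeginPlay, whose curves drive the mesh's relative Z and the Scene component's scale.
; The scale curve multiplies the mesh's world scale captured in the construction script.
; It always reports that it can be interacted with and never that it can be swapped.
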(event EventBeginPlay
  (Components|Timeline|SetPlayRate (Variables|Default|GetTimeline) 4.0))

(event Collision|EventActorBeginOverlap
  (params (OtherActor :type Actor%20Object%20Reference)))

(event EventTick
  (params (DeltaSeconds :type Float%20%28single-precision%29)))

(event EventInteract
  (params (Hit%20Component :type Primitive%20Component%20Object%20Reference))
  (bind (_direction _height _rotation _scale) (Timeline|Timeline PlayFromStart)
    (:Update
      (Transformation|SetRelativeTransform (Variables|Default|GetStaticMesh) (Math|Transform|MakeTransform (Math|Vector|MakeVector 0.0 0.0 _height) "0, 0, 0" "1.000000,1.000000,1.000000") false false)
      (Transformation|SetRelativeScale3D (Variables|Default|GetScene) (* (Math|Conversions|ToVector(Float) _scale) (Variables|Default|GetInitial%20Scale))))))

(fn ConstructionScript
  (Variables|Default|SetInitial%20Scale (Transformation|GetWorldScale (Variables|Default|GetStaticMesh))))

(fn GetCanInteract
  (return true))

(fn GetCanSwap
  (return false))