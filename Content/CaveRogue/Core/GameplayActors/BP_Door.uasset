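; BP_Door is an interactable door that rotates its static mesh in yaw between zero and OpenAngle.
; Interact plays or reverses the OpenCloseDoor timeline based on the Open flag, then flips the flag, with timeline updates lerping the yaw.
; The construction script sets the initial rotation from Open.
; Interaction queries report that it can always be interacted with and never swapped.
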(event EventBeginPlay)

(event EventTick
  (params (DeltaSeconds :type Float%20%28single-precision%29)))

(event EventInteract
  (params (Hit%20Component :type Primitive%20Component%20Object%20Reference))
  (Utilities|FlowControl|Sequence
    (:then_0
      (if (Variables|Default|GetOpen)
        (bind _rotation (Timeline|Open/Close%20Door Play)
          (:Update
            (Transformation|SetRelativeRotation (Variables|Default|GetStaticMesh) (Math|Rotator|MakeRotator 0.0 0.0 (Math|Float|Lerp 0.0 (Variables|Default|GetOpen%20Angle) _rotation)) false false)))
        (else
          (Timeline|Open/Close%20Door Reverse))))
    (:then_1
      (Variables|Default|SetOpen (not (Variables|Default|GetOpen))))))

(fn ConstructionScript
  (Transformation|SetRelativeRotation (Variables|Default|GetStaticMesh) (Math|Rotator|MakeRotator 0.0 0.0 (Math|Float|SelectFloat (Variables|Default|GetOpen%20Angle) 0.0 (Variables|Default|GetOpen))) false false))

(fn GetCanInteract
  (return true))

(fn GetCanSwap
  (return false))