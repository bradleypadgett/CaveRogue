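; BP_Target is an interactable target prop that shows accumulated hits through its red and white emissive materials.
; DamageTarget counts hits, weighting the Bullseye component as three, and uses that count to set color-mask hardness and radius on dynamic material instances created in the construction script.
; Interact resets the count and visuals, then plays a sped-up timeline that animates the scale relative to the cached construction-time scale.
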(event EventBeginPlay
  (Components|Timeline|SetPlayRate (Variables|Default|GetTimeline) 4.0))

(event Collision|EventActorBeginOverlap
  (params (OtherActor :type Actor%20Object%20Reference)))

(event EventTick
  (params (DeltaSeconds :type Float%20%28single-precision%29)))

(event EventInteract
  (params (Hit%20Component :type Primitive%20Component%20Object%20Reference))
  (Variables|Default|SetHits 0)
  (Utilities|FlowControl|Sequence
    (:then_0
      (Rendering|Material|SetScalarParameterValue (Variables|Default|GetTarget%20White) "Color Mask Hardness" (Math|Float|SelectFloat 0.0 (Utilities|Select :Index (Variables|Default|GetHits) :Option%200 1.0 :Option%201 0.1 :Option%202 0.04 :Option%203 0.0) (> (Variables|Default|GetHits) 3)) :!class /Script/Engine.MaterialInstanceDynamic)
      (Rendering|Material|SetScalarParameterValue (Variables|Default|GetTarget%20Red) "Color Mask Radius" (Math|Float|SelectFloat 0.6 (Utilities|Select :Index (Variables|Default|GetHits) :Option%200 1.0 :Option%201 4.0 :Option%202 2.0 :Option%203 1.0) (> (Variables|Default|GetHits) 3)) :!class /Script/Engine.MaterialInstanceDynamic)
      (Rendering|Material|SetScalarParameterValue (Variables|Default|GetTarget%20White) "Color Mask Radius" (Math|Float|SelectFloat 0.5 (Utilities|Select :Index (Variables|Default|GetHits) :Option%200 1.0 :Option%201 3.75 :Option%202 4.0 :Option%203 1.0) (> (Variables|Default|GetHits) 3)) :!class /Script/Engine.MaterialInstanceDynamic))
    (:then_1
      (bind _scale (Timeline|Timeline PlayFromStart)
        (:Update
          (Transformation|SetRelativeScale3D (Variables|Default|GetScene) (* (Math|Conversions|ToVector(Float) _scale) (Variables|Default|GetScale))))))))

(event EventDamageTarget
  (params (Hit%20Component :type Primitive%20Component%20Object%20Reference))
  (Utilities|FlowControl|Sequence
    (:then_0
      (if (== Hit%20Component (Variables|Default|GetBullseye))
        (Variables|Default|SetHits (+ (Variables|Default|GetHits) 3))
        (else
          (Math|Integer|IncrementInt (Variables|Default|GetHits)))))
    (:then_1
      (Rendering|Material|SetScalarParameterValue (Variables|Default|GetTarget%20White) "Color Mask Hardness" (Math|Float|SelectFloat 0.0 (Utilities|Select :Index (Variables|Default|GetHits) :Option%200 1.0 :Option%201 0.1 :Option%202 0.04 :Option%203 0.0) (> (Variables|Default|GetHits) 3)) :!class /Script/Engine.MaterialInstanceDynamic)
      (Rendering|Material|SetScalarParameterValue (Variables|Default|GetTarget%20Red) "Color Mask Radius" (Math|Float|SelectFloat 0.6 (Utilities|Select :Index (Variables|Default|GetHits) :Option%200 1.0 :Option%201 4.0 :Option%202 2.0 :Option%203 1.0) (> (Variables|Default|GetHits) 3)) :!class /Script/Engine.MaterialInstanceDynamic)
      (Rendering|Material|SetScalarParameterValue (Variables|Default|GetTarget%20White) "Color Mask Radius" (Math|Float|SelectFloat 0.5 (Utilities|Select :Index (Variables|Default|GetHits) :Option%200 1.0 :Option%201 3.75 :Option%202 4.0 :Option%203 1.0) (> (Variables|Default|GetHits) 3)) :!class /Script/Engine.MaterialInstanceDynamic))))

(fn ConstructionScript
  (bind _staticmesh (Variables|Default|GetStaticMesh))
  (bind _staticmesh_2 (Variables|Default|GetStaticMesh))
  (Utilities|FlowControl|Sequence
    (:then_0
      (bind _returnvalue (Rendering|Material|CreateDynamicMaterialInstance _staticmesh_2 1 "/Game/CaveRogue/Props/MI_PropColor_Red_Emissive.MI_PropColor_Red_Emissive" "None" :!class /Script/Engine.PrimitiveComponent))
      (bind _output_get (Variables|Default|SetTarget%20Red _returnvalue))
      (Rendering|Material|SetMaterial _staticmesh_2 1 _output_get)
      (bind _returnvalue_2 (Rendering|Material|CreateDynamicMaterialInstance _staticmesh 2 "/Game/CaveRogue/Props/MI_PropColor_White_Emissive.MI_PropColor_White_Emissive" "None" :!class /Script/Engine.PrimitiveComponent))
      (bind _output_get_2 (Variables|Default|SetTarget%20White _returnvalue_2))
      (Rendering|Material|SetMaterial _staticmesh 2 _output_get_2))
    (:then_1
      (Variables|Default|SetScale (Transformation|GetWorldScale (Variables|Default|GetScene))))))

(fn GetCanDamage
  (return false))

(fn GetCanInteract
  (return true))